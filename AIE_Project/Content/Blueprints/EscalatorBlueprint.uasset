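; Escalator actor that moves a loop of cube steps along a spline.
; The construction script spawns static mesh steps at StepDistance intervals along the spline and records each one's distance.
; Each Tick places every step at its stored distance, then advances it by Speed, resetting to zero past the spline's end.
; Movement is per frame, without delta-time scaling, and updates only location.
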(event `self.ReceiveTick`
  (params (DeltaSeconds :type "Float (single-precision)"))
  (bind _current_distance (`self.Current distance`))
  (for (_array_element _array_index) (`self.Steps`)
    (bind _output (`|GetArrayItem` _current_distance _array_index))
    (`SceneComponent.K2_SetWorldLocation` _array_element (`SplineComponent.GetLocationAtDistanceAlongSpline` (`self.Spline`) _output "World") false false)
    (bind _returnvalue (+ _output (`self.Speed`)))
    (`/Engine/EditorBlueprintResources/StandardMacros.CompareFloat` _returnvalue (`SplineComponent.GetSplineLength` (`self.Spline`))
      (:`>`
        (`KismetArrayLibrary.Array_Set` _current_distance _array_index 0.0 true))
      (:`<`
        (`KismetArrayLibrary.Array_Set` _current_distance _array_index _returnvalue true)))))

(fn `UserConstructionScript`
  (bind _spline (`self.Spline`))
  (bind _step_distance (`self.Step distance`))
  (for _index (range (+ (`.ReturnValue` (`KismetMathLibrary.FMod` (`SplineComponent.GetSplineLength` _spline) _step_distance)) 1))
    (bind _returnvalue (* _index _step_distance))
    (`KismetArrayLibrary.Array_Add` (`self.Current distance`) _returnvalue)
    (bind _returnvalue_2 (`AddComponent|NODE_AddStaticMeshComponent-0` :`bManualAttachment` true :`RelativeTransform` (`KismetMathLibrary.MakeTransform` (`SplineComponent.GetLocationAtDistanceAlongSpline` _spline _returnvalue "World") (struct :`Yaw` 90.0))))
    (`StaticMeshComponent.SetStaticMesh` _returnvalue_2 "/Game/StarterContent/Shapes/Shape_Cube.Shape_Cube")
    (`PrimitiveComponent.SetMaterial` _returnvalue_2 0 "/Game/StarterContent/Props/Materials/M_MaterialSphere.M_MaterialSphere")
    (`KismetArrayLibrary.Array_Add` (`self.Steps`) _returnvalue_2)))